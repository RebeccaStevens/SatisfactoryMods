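; Drag-and-drop operation for reordering list elements in the BBW ReorderList widget.
; While dragged, it moves the payload item live within the list view to the drop index computed from the pointer's position in list-local space.
; A drop, or a cancelled drag without right mouse held, ends the drag and reports whether the index changed.
; Cancelling with right mouse held asks the element to reset to its original index.
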(event EventDrop
  (params (PointerEvent :type Pointer%20Event%20Structure%20%28by%20ref%29))
  (Variables|Default|Set%28Internal%29%20Should%20Cancel false)
  (bind _index (Default|GetIndexinList (Variables|Default|GetElement)))
  (if (Variables|Default|Get%28Internal%29%20Should%20Cancel)
    (Default|CancelDrag (Variables|Default|GetElement) (Variables|Default|GetOriginal%20Index) _index)
    (else
      (Default|EndDrag (Variables|Default|GetElement) (!= (Variables|Default|GetOriginal%20Index) _index)))))

(event EventDragCancelled
  (params (PointerEvent :type Pointer%20Event%20Structure%20%28by%20ref%29))
  (Variables|Default|Set%28Internal%29%20Should%20Cancel (Class|KismetInputLibrary|PointerEventIsMouseButtonDown PointerEvent "RightMouseButton"))
  (bind _index (Default|GetIndexinList (Variables|Default|GetElement)))
  (if (Variables|Default|Get%28Internal%29%20Should%20Cancel)
    (Default|CancelDrag (Variables|Default|GetElement) (Variables|Default|GetOriginal%20Index) _index)
    (else
      (Default|EndDrag (Variables|Default|GetElement) (!= (Variables|Default|GetOriginal%20Index) _index)))))

(event EventDragged
  (params (PointerEvent :type Pointer%20Event%20Structure%20%28by%20ref%29))
  (bind (_drop_index _is_over_list _list_view) (Utilities|DragEventStatus PointerEvent))
  (Class|BBWUtils|MoveIteminListView _list_view (Class|ListView|GetIndexforItem _list_view (Variables|Default|GetPayload)) _drop_index))