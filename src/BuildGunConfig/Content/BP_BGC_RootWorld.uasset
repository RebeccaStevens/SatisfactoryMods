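; BP_BGC_RootWorld is a world module that hooks saved configuration into the BGC player subsystem.
; During the Construction lifecycle phase it fetches that subsystem actor and loads build mode data from a serialized JSON config property.
; It also binds the equipment layout property's value-changed event, so edits make the subsystem update the player's equipment inventory positions.
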(event Custom|Update%20Player%20Equipment%20Inventory%20Positions
  (Default|UpdatePlayerEquipmentInventoryPositions (Class|SubsystemActorManager|GetSubsystemActor (Subsystems|GetSubsystemActorManager) "/BuildGunConfig/BP_BGC_PlayerSubsystem.BP_BGC_PlayerSubsystem_C")))

(event EventOnLifecycleEvent
  (params (Phase :type ELifecyclePhase%20Enum :default "CONSTRUCTION"))
  (switch Utilities|FlowControl|Switch|SwitchonELifecyclePhase Phase
    (:CONSTRUCTION
      (Variables|Default|SetPlayerSubsystem (Class|SubsystemActorManager|GetSubsystemActor (Subsystems|GetSubsystemActorManager) "/BuildGunConfig/BP_BGC_PlayerSubsystem.BP_BGC_PlayerSubsystem_C"))
      (Utilities|FlowControl|Sequence
        (:then_0
          (bind _config_property (CallFunction|GetBuildModesSerializedConfigProperty))
          (Class|BGCAbstractPlayerSubsystem|LoadBuildModeDatafromJsonString (Variables|Default|GetPlayerSubsystem) (Variables|/Script/SML.ConfigPropertyString|GetValue _config_property)))
        (:then_1
          (bind _config_property_2 (CallFunction|GetEquipmentLayoutConfigProperty))
          (EventDispatchers|BindEventtoOnPropertyValueChanged _config_property_2 (delegate Custom|Update%20Player%20Equipment%20Inventory%20Positions)))))))