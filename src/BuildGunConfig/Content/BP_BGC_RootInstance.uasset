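; BGC root instance that supplies position data for the equipment slots in the player inventory, including a Build Gun slot.
; GetLayoutData switches on the layout option to return either the vanilla insert-only arrangement or one of two full rearrangements.
; Each layout builder fills a struct giving anchors, position, alignment and label justification for head, body, back, hands, legs and build gun.
; Positions come from shared column and row variables.
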(fn GetLayoutData
  (params (Layout%20Option :type BPE_BGC_PlayerInventoryEquipment_Layouts%20Enum :default "NewEnumerator0"))
  (switch Utilities|FlowControl|Switch|SwitchonBPE_BGC_PlayerInventoryEquipment_Layouts Layout%20Option
    (:NewEnumerator1
      (return (BuildGunConfig|GetLayoutVanilla)))
    (:NewEnumerator2
      (return (BuildGunConfig|GetLayout1)))
    (:NewEnumerator0
      (return (BuildGunConfig|GetLayout2)))))

(fn GetLayoutVanilla
  (return (Utilities|Struct|MakeBPS_BGC_PlayerInventoryEquipment_PositionData (Utilities|Struct|MakeBPS_BGC_PlayerInventoryEquipment_Element_PositionData (LocalVariables|GetAnchors) (Math|Vector2D|MakeVector2D (LocalVariables|GetLeft) (LocalVariables|GetRow%201)) "(X=0.000000,Y=0.500000)" "HAlign_Left") (Utilities|Struct|MakeBPS_BGC_PlayerInventoryEquipment_Element_PositionData (LocalVariables|GetAnchors) (Math|Vector2D|MakeVector2D (LocalVariables|GetRight) (LocalVariables|GetRow%201)) "(X=1.000000,Y=0.500000)" "HAlign_Right") (Utilities|Struct|MakeBPS_BGC_PlayerInventoryEquipment_Element_PositionData (LocalVariables|GetAnchors) (Math|Vector2D|MakeVector2D (LocalVariables|GetRight) (LocalVariables|GetRow%202)) "(X=1.000000,Y=0.500000)" "HAlign_Right") (Utilities|Struct|MakeBPS_BGC_PlayerInventoryEquipment_Element_PositionData (LocalVariables|GetAnchors) (Math|Vector2D|MakeVector2D (LocalVariables|GetLeft) (LocalVariables|GetRow%202)) "(X=0.000000,Y=0.500000)" "HAlign_Left") (Utilities|Struct|MakeBPS_BGC_PlayerInventoryEquipment_Element_PositionData (LocalVariables|GetAnchors) (Math|Vector2D|MakeVector2D (LocalVariables|GetLeft) (LocalVariables|GetRow%203)) "(X=0.000000,Y=0.500000)" "HAlign_Left") (Utilities|Struct|MakeBPS_BGC_PlayerInventoryEquipment_Element_PositionData (LocalVariables|GetAnchors) (Math|Vector2D|MakeVector2D (LocalVariables|GetRight) (LocalVariables|GetRow%203)) "(X=1.000000,Y=0.500000)" "HAlign_Right"))))

(fn GetLayout1
  (return (Utilities|Struct|MakeBPS_BGC_PlayerInventoryEquipment_PositionData (Utilities|Struct|MakeBPS_BGC_PlayerInventoryEquipment_Element_PositionData (LocalVariables|GetAnchors) (Math|Vector2D|MakeVector2D (LocalVariables|GetRight) (LocalVariables|GetRow%201)) "(X=1.000000,Y=0.500000)" "HAlign_Right") (Utilities|Struct|MakeBPS_BGC_PlayerInventoryEquipment_Element_PositionData (LocalVariables|GetAnchors) (Math|Vector2D|MakeVector2D (LocalVariables|GetLeft) (LocalVariables|GetRow%202)) "(X=0.000000,Y=0.500000)" "HAlign_Left") (Utilities|Struct|MakeBPS_BGC_PlayerInventoryEquipment_Element_PositionData (LocalVariables|GetAnchors) (Math|Vector2D|MakeVector2D (LocalVariables|GetRight) (LocalVariables|GetRow%203)) "(X=1.000000,Y=0.500000)" "HAlign_Right") (Utilities|Struct|MakeBPS_BGC_PlayerInventoryEquipment_Element_PositionData (LocalVariables|GetAnchors) (Math|Vector2D|MakeVector2D (LocalVariables|GetLeft) (LocalVariables|GetRow%204)) "(X=0.000000,Y=0.500000)" "HAlign_Left") (Utilities|Struct|MakeBPS_BGC_PlayerInventoryEquipment_Element_PositionData (LocalVariables|GetAnchors) (Math|Vector2D|MakeVector2D (LocalVariables|GetLeft) (LocalVariables|GetRow%206)) "(X=0.000000,Y=0.500000)" "HAlign_Left") (Utilities|Struct|MakeBPS_BGC_PlayerInventoryEquipment_Element_PositionData (LocalVariables|GetAnchors) (Math|Vector2D|MakeVector2D (LocalVariables|GetRight) (LocalVariables|GetRow%205)) "(X=1.000000,Y=0.500000)" "HAlign_Right"))))

(fn GetLayout2
  (return (Utilities|Struct|MakeBPS_BGC_PlayerInventoryEquipment_PositionData (Utilities|Struct|MakeBPS_BGC_PlayerInventoryEquipment_Element_PositionData (LocalVariables|GetAnchors) (Math|Vector2D|MakeVector2D (LocalVariables|GetCenter) (LocalVariables|GetRow%201)) "(X=0.500000,Y=0.500000)" "HAlign_Center") (Utilities|Struct|MakeBPS_BGC_PlayerInventoryEquipment_Element_PositionData (LocalVariables|GetAnchors) (Math|Vector2D|MakeVector2D (LocalVariables|GetLeft) (LocalVariables|GetRow%202)) "(X=0.000000,Y=0.500000)" "HAlign_Left") (Utilities|Struct|MakeBPS_BGC_PlayerInventoryEquipment_Element_PositionData (LocalVariables|GetAnchors) (Math|Vector2D|MakeVector2D (LocalVariables|GetRight) (LocalVariables|GetRow%202)) "(X=1.000000,Y=0.500000)" "HAlign_Right") (Utilities|Struct|MakeBPS_BGC_PlayerInventoryEquipment_Element_PositionData (LocalVariables|GetAnchors) (Math|Vector2D|MakeVector2D (LocalVariables|GetLeft) (LocalVariables|GetRow%203)) "(X=0.000000,Y=0.000000)" "HAlign_Left") (Utilities|Struct|MakeBPS_BGC_PlayerInventoryEquipment_Element_PositionData (LocalVariables|GetAnchors) (Math|Vector2D|MakeVector2D (LocalVariables|GetLeft) (LocalVariables|GetRow%204)) "(X=0.000000,Y=0.500000)" "HAlign_Left") (Utilities|Struct|MakeBPS_BGC_PlayerInventoryEquipment_Element_PositionData (LocalVariables|GetAnchors) (Math|Vector2D|MakeVector2D (LocalVariables|GetRight) (LocalVariables|GetRow%203)) "(X=1.000000,Y=0.000000)" "HAlign_Right"))))