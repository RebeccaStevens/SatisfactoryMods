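; Player subsystem that drives build gun configuration panels inside the player's equipment inventory window.
; Setup caches widgets, rebuilds build mode groups and binds buttons that open config panels via a widget switcher with history-based back navigation.
; Panels are sized to the switcher before display, and build mode edits trigger a save.
; It also supplies selectable equipment slot layouts and config-backed defaults for nudging, rotation and locked-buildable visibility.
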(event Custom|Set%20Up%20Build%20Gun%20Inventory
  (params (Window :type Widget%20Window%20Dark%20Mode%20Object%20Reference) (Build%20Gun%20Widget :type BPW%20BGC%20Equipment%20Slot%20Object%20Reference) (Equipment%20Panel%20Wrapper :type BPW%20BGC%20Equipment%20Wrapper%20Object%20Reference) (Layout%20Button :type BPW%20BGC%20Equipment%20Layout%20Menu%20Button%20Object%20Reference) (Build%20Gun%20Config%20Widgets%20Map :type Map%20of%20BPW%20BGC%20Config%20Panel%20Class%20References%20to%20Integers))
  (|SetVariables Window Build%20Gun%20Widget Equipment%20Panel%20Wrapper Layout%20Button Build%20Gun%20Config%20Widgets%20Map)
  (Utilities|FlowControl|Sequence
    (:then_0
      (Utilities|ResetNavigationHistory (Utilities|Struct|MakeBGC_NavigationHistoryEntry))
      (Class|BGCAbstractPlayerSubsystem|RebuildBuildModeGroups))
    (:then_1
      (Utilities|FlowControl|Sequence
        (:then_0
          (bind (_widget _index _widget_class) (Utilities|BuildGunConfigWidget))
          (EventDispatchers|BindEventtoSwitchtoEditBuildMode _widget (delegate Custom|Open%20Build%20Gun%20Build%20Mode%20Config))
          (Default|ClearBuildModes (Variables|/BuildGunConfig/Widgets/BuildGunConfig/Index/BPW_BGC_BuildGunConfig.BPW_BGC_BuildGunConfig_C|GetGroupBuildModesContent _widget))
          (for _array_element (Class|BGCAbstractPlayerSubsystem|GetBuildModeGroupIdsforDisplay)
            (Default|AddBuildModeGroup (Variables|/BuildGunConfig/Widgets/BuildGunConfig/Index/BPW_BGC_BuildGunConfig.BPW_BGC_BuildGunConfig_C|GetGroupBuildModesContent _widget) _array_element)))
        (:then_1
          (EventDispatchers|BindEventtoBuildGunSettingButtonClicked (Variables|BuildGunConfig|GetBuild%20Gun%20Widget) (delegate Custom|Open%20Build%20Gun%20Config)))))))

(event Custom|Update%20Player%20Equipment%20Inventory%20Positions
  (bind _returnvalue (Class|FGBlueprintFunctionLibrary|GetFirstChildWidgetOfClass (Variables|BuildGunConfig|GetWindow) "/Game/FactoryGame/Character/Player/Widget_PlayerEquipmentInventory.Widget_PlayerEquipmentInventory_C"))
  (CallFunction|UpdatePlayerEquipmentInventoryPositions(internal) _returnvalue (Variables|BuildGunConfig|GetBuild%20Gun%20Widget) (Variables|BuildGunConfig|GetEquipment%20Layout%20Button)))

(event Custom|Build%20Mode%20Data%20Changed
  (Class|BGCAbstractPlayerSubsystem|SaveBuildModeData))

(event Custom|Close%20Build%20Gun%20Config
  (bind _bgc_navigationhistoryentry (Utilities|Struct|MakeBGC_NavigationHistoryEntry))
  (Utilities|ResetNavigationHistory _bgc_navigationhistoryentry)
  (BuildGunConfig|SetEquipmentWidgetChild _bgc_navigationhistoryentry))

(event Custom|Open%20Build%20Gun%20Build%20Mode%20Config
  (params (Build%20Mode%20Group%20Id :type Integer))
  (bind (_widget _index _widget_class) (Utilities|BuildModeConfigWidget))
  (BuildGunConfig|EnsureSize (Variables|/BuildGunConfig/Widgets/EquipmentPanel/BPW_BGC_Equipment_Wrapper.BPW_BGC_Equipment_Wrapper_C|GetFGWidgetSwitcher (Variables|BuildGunConfig|GetEquipment%20Panel%20Wrapper)) _index)
  (BuildGunConfig|Navigateto _widget_class (Class|BGCNavigationHistoryEntryDataBuildModeGroupId|Make Build%20Mode%20Group%20Id))
  (EventDispatchers|BindEventtoOnDataChanged _widget (delegate Custom|Build%20Mode%20Data%20Changed)))

(event Custom|Open%20Build%20Gun%20Config
  (BuildGunConfig|EnsureSize (Variables|/BuildGunConfig/Widgets/EquipmentPanel/BPW_BGC_Equipment_Wrapper.BPW_BGC_Equipment_Wrapper_C|GetFGWidgetSwitcher (Variables|BuildGunConfig|GetEquipment%20Panel%20Wrapper)) (stale Custom|Set%20Up%20Build%20Gun%20Inventory _index))
  (BuildGunConfig|Navigateto (stale Custom|Set%20Up%20Build%20Gun%20Inventory _widget_class)))

(fn ConstructionScript)

(fn GetWidgetSwitcher
  (params (EquipmentPanelWrapperWidget :type FG%20User%20Widget%20Object%20Reference))
  (bind _asbpw_bgc_equipment_wrapper (Utilities|Casting|CastToBPW_BGC_Equipment_Wrapper EquipmentPanelWrapperWidget)
    (:then
      (return (Variables|/BuildGunConfig/Widgets/EquipmentPanel/BPW_BGC_Equipment_Wrapper.BPW_BGC_Equipment_Wrapper_C|GetFGWidgetSwitcher _asbpw_bgc_equipment_wrapper)))
    (:CastFailed
      (Class|BlueprintLoggingLibrary|LogError "Unexpected data type"))))

(fn EnsureSize
  (params (Switcher :type Widget%20Switcher%20Object%20Reference) (Config%20Index :type Integer))
  (bind _returnvalue (Class|Widget|GetCachedGeometry Switcher))
  (bind _returnvalue_2 (Class|SlateBlueprintLibrary|GetLocalSize _returnvalue))
  (bind (_x _y) (Math|Vector2D|BreakVector2D _returnvalue_2))
  (bind _asbpw_bgc_config_panel (Utilities|Casting|CastToBPW_BGC_ConfigPanel (Class|WidgetSwitcher|GetWidgetatIndex Switcher Config%20Index)))
  (Variables|/Script/UMG.SizeBox|SetWidthOverride (Variables|/BuildGunConfig/Widgets/BuildGunConfig/Index/BPW_BGC_BuildGunConfig.BPW_BGC_BuildGunConfig_C|GetContainerSize _asbpw_bgc_config_panel) _x)
  (Variables|/Script/UMG.SizeBox|SetHeightOverride (Variables|/BuildGunConfig/Widgets/BuildGunConfig/Index/BPW_BGC_BuildGunConfig.BPW_BGC_BuildGunConfig_C|GetContainerSize _asbpw_bgc_config_panel) _y))

(fn GetActiveEquipmentLayout
  (bind _config_property (CallFunction|GetEquipmentLayoutConfigProperty))
  (return (Utilities|Enum|ByteToEnumBPE_BGC_PlayerInventoryEquipment_Layouts (Math|Conversions|ToByte(Integer) (Class|RuntimeBlueprintFunctionLibrary|ToInteger(ConfigProperty) _config_property)))))

(fn GetActiveEquipmentLayoutData
  (bind _layout (BuildGunConfig|EquipmentLayout|GetActiveEquipmentLayout))
  (return (BuildGunConfig|EquipmentLayout|GetEquipmentLayoutData _layout)))

(fn GetEquipmentLayoutData
  (params (Layout%20Option :type BPE_BGC_PlayerInventoryEquipment_Layouts%20Enum :default "NewEnumerator0"))
  (switch Utilities|FlowControl|Switch|SwitchonBPE_BGC_PlayerInventoryEquipment_Layouts Layout%20Option
    (:NewEnumerator1
      (return (BuildGunConfig|EquipmentLayout|GetEquipmentLayoutVanilla)))
    (:NewEnumerator2
      (return (BuildGunConfig|EquipmentLayout|GetEquipmentLayout1)))
    (:NewEnumerator0
      (return (BuildGunConfig|EquipmentLayout|GetEquipmentLayout2)))))

(fn GetEquipmentLayoutVanilla
  (return (Utilities|Struct|MakeBPS_BGC_PlayerInventoryEquipment_PositionData (Utilities|Struct|MakeBPS_BGC_PlayerInventoryEquipment_Element_PositionData (LocalVariables|GetAnchors) (Math|Vector2D|MakeVector2D (LocalVariables|GetLeft) (LocalVariables|GetRow%201)) "(X=0.000000,Y=0.500000)" "HAlign_Left") (Utilities|Struct|MakeBPS_BGC_PlayerInventoryEquipment_Element_PositionData (LocalVariables|GetAnchors) (Math|Vector2D|MakeVector2D (LocalVariables|GetRight) (LocalVariables|GetRow%201)) "(X=1.000000,Y=0.500000)" "HAlign_Right") (Utilities|Struct|MakeBPS_BGC_PlayerInventoryEquipment_Element_PositionData (LocalVariables|GetAnchors) (Math|Vector2D|MakeVector2D (LocalVariables|GetRight) (LocalVariables|GetRow%202)) "(X=1.000000,Y=0.500000)" "HAlign_Right") (Utilities|Struct|MakeBPS_BGC_PlayerInventoryEquipment_Element_PositionData (LocalVariables|GetAnchors) (Math|Vector2D|MakeVector2D (LocalVariables|GetLeft) (LocalVariables|GetRow%202)) "(X=0.000000,Y=0.500000)" "HAlign_Left") (Utilities|Struct|MakeBPS_BGC_PlayerInventoryEquipment_Element_PositionData (LocalVariables|GetAnchors) (Math|Vector2D|MakeVector2D (LocalVariables|GetLeft) (LocalVariables|GetRow%203)) "(X=0.000000,Y=0.500000)" "HAlign_Left") (Utilities|Struct|MakeBPS_BGC_PlayerInventoryEquipment_Element_PositionData (LocalVariables|GetAnchors) (Math|Vector2D|MakeVector2D (LocalVariables|GetRight) (LocalVariables|GetRow%203)) "(X=1.000000,Y=0.500000)" "HAlign_Right"))))

(fn GetEquipmentLayout1
  (return (Utilities|Struct|MakeBPS_BGC_PlayerInventoryEquipment_PositionData (Utilities|Struct|MakeBPS_BGC_PlayerInventoryEquipment_Element_PositionData (LocalVariables|GetAnchors) (Math|Vector2D|MakeVector2D (LocalVariables|GetRight) (LocalVariables|GetRow%201)) "(X=1.000000,Y=0.500000)" "HAlign_Right") (Utilities|Struct|MakeBPS_BGC_PlayerInventoryEquipment_Element_PositionData (LocalVariables|GetAnchors) (Math|Vector2D|MakeVector2D (LocalVariables|GetLeft) (LocalVariables|GetRow%202)) "(X=0.000000,Y=0.500000)" "HAlign_Left") (Utilities|Struct|MakeBPS_BGC_PlayerInventoryEquipment_Element_PositionData (LocalVariables|GetAnchors) (Math|Vector2D|MakeVector2D (LocalVariables|GetRight) (LocalVariables|GetRow%203)) "(X=1.000000,Y=0.500000)" "HAlign_Right") (Utilities|Struct|MakeBPS_BGC_PlayerInventoryEquipment_Element_PositionData (LocalVariables|GetAnchors) (Math|Vector2D|MakeVector2D (LocalVariables|GetLeft) (LocalVariables|GetRow%204)) "(X=0.000000,Y=0.500000)" "HAlign_Left") (Utilities|Struct|MakeBPS_BGC_PlayerInventoryEquipment_Element_PositionData (LocalVariables|GetAnchors) (Math|Vector2D|MakeVector2D (LocalVariables|GetLeft) (LocalVariables|GetRow%206)) "(X=0.000000,Y=0.500000)" "HAlign_Left") (Utilities|Struct|MakeBPS_BGC_PlayerInventoryEquipment_Element_PositionData (LocalVariables|GetAnchors) (Math|Vector2D|MakeVector2D (LocalVariables|GetRight) (LocalVariables|GetRow%205)) "(X=1.000000,Y=0.500000)" "HAlign_Right"))))

(fn GetEquipmentLayout2
  (return (Utilities|Struct|MakeBPS_BGC_PlayerInventoryEquipment_PositionData (Utilities|Struct|MakeBPS_BGC_PlayerInventoryEquipment_Element_PositionData (LocalVariables|GetAnchors) (Math|Vector2D|MakeVector2D (LocalVariables|GetCenter) (LocalVariables|GetRow%201)) "(X=0.500000,Y=0.500000)" "HAlign_Center") (Utilities|Struct|MakeBPS_BGC_PlayerInventoryEquipment_Element_PositionData (LocalVariables|GetAnchors) (Math|Vector2D|MakeVector2D (LocalVariables|GetLeft) (LocalVariables|GetRow%202)) "(X=0.000000,Y=0.500000)" "HAlign_Left") (Utilities|Struct|MakeBPS_BGC_PlayerInventoryEquipment_Element_PositionData (LocalVariables|GetAnchors) (Math|Vector2D|MakeVector2D (LocalVariables|GetRight) (LocalVariables|GetRow%202)) "(X=1.000000,Y=0.500000)" "HAlign_Right") (Utilities|Struct|MakeBPS_BGC_PlayerInventoryEquipment_Element_PositionData (LocalVariables|GetAnchors) (Math|Vector2D|MakeVector2D (LocalVariables|GetLeft) (LocalVariables|GetRow%203)) "(X=0.000000,Y=0.000000)" "HAlign_Left") (Utilities|Struct|MakeBPS_BGC_PlayerInventoryEquipment_Element_PositionData (LocalVariables|GetAnchors) (Math|Vector2D|MakeVector2D (LocalVariables|GetLeft) (LocalVariables|GetRow%204)) "(X=0.000000,Y=0.500000)" "HAlign_Left") (Utilities|Struct|MakeBPS_BGC_PlayerInventoryEquipment_Element_PositionData (LocalVariables|GetAnchors) (Math|Vector2D|MakeVector2D (LocalVariables|GetRight) (LocalVariables|GetRow%203)) "(X=1.000000,Y=0.000000)" "HAlign_Right"))))

(fn SetEquipmentWidgetChild
  (params (Child%20Data :type BGC%20Navigation%20History%20Entry%20Structure))
  (bind (_index _data) (Utilities|Struct|BreakBGC_NavigationHistoryEntry Child%20Data))
  (bind _equipment_panel_wrapper (Variables|BuildGunConfig|GetEquipment%20Panel%20Wrapper))
  (bind _fgwidgetswitcher (Variables|/BuildGunConfig/Widgets/EquipmentPanel/BPW_BGC_Equipment_Wrapper.BPW_BGC_Equipment_Wrapper_C|GetFGWidgetSwitcher _equipment_panel_wrapper))
  (if (and (>= _index 0) (< _index (Class|WidgetSwitcher|GetNumWidgets _fgwidgetswitcher)))
    (Utilities|FlowControl|Sequence
      (:then_0
        (Class|WidgetSwitcher|SetActiveWidgetIndex _fgwidgetswitcher _index)
        (bind _asbpw_bgc_config_panel (Utilities|Casting|CastToBPW_BGC_ConfigPanel (Class|WidgetSwitcher|GetActiveWidget _fgwidgetswitcher)))
        (Default|Initialize _asbpw_bgc_config_panel _data)))
    (else
      (Class|BlueprintLoggingLibrary|LogError (Utilities|String|Append "Invalid Index: " (Utilities|String|ToString(Integer) _index))))))

(fn NavigateBack
  (bind _navigationhistory (Variables|Default|GetNavigationHistory))
  (bind _returnvalue (Utilities|Array|LastIndex _navigationhistory))
  (BuildGunConfig|SetEquipmentWidgetChild (Utilities|Array|Get(acopy) _navigationhistory (- _returnvalue 1)))
  (Utilities|Array|RemoveIndex _navigationhistory _returnvalue))

(fn Navigateto
  (params (To :type BPW%20BGC%20Config%20Panel%20Class%20Reference) (Data :type BGC%20Navigation%20History%20Entry%20Data%20Object%20Reference))
  (bind _build_gun_config_widgets_map (Variables|BuildGunConfig|GetBuild%20Gun%20Config%20Widgets%20Map))
  (bind (_value _returnvalue) (Utilities|Map|Find _build_gun_config_widgets_map To))
  (bind _bgc_navigationhistoryentry (Utilities|Struct|MakeBGC_NavigationHistoryEntry _value Data))
  (if _returnvalue
    (BuildGunConfig|SetEquipmentWidgetChild _bgc_navigationhistoryentry)
    (Utilities|Array|Add (Variables|Default|GetNavigationHistory) _bgc_navigationhistoryentry)
    (else
      (Class|BlueprintLoggingLibrary|LogError (Utilities|String|Append "Item Not Found: " (Utilities|GetClassDisplayName To))))))

(fn ShouldShowLockedBuildables
  (bind _config_property (CallFunction|GetShowLockedConfigProperty))
  (return (Class|RuntimeBlueprintFunctionLibrary|ToBoolean(ConfigPropertyBool) _config_property)))

(fn GetDefaultNudgeDistance
  (bind _config_property (CallFunction|GetNudgingDefaultConfigProperty))
  (return (Class|RuntimeBlueprintFunctionLibrary|ToFloat(ConfigProperty) _config_property)))

(fn GetDefaultRotationStep
  (bind _config_property (CallFunction|GetRotationSnapDefaultConfigProperty))
  (return (Class|RuntimeBlueprintFunctionLibrary|ToInteger(ConfigPropertyInteger) _config_property)))